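; BP_Player is the top-down RPG player pawn, handling Enhanced Input movement and dialogue-style interaction.
; Interact sends an interface message to the first overlapping actor, or while interaction is locked, instantly reveals or advances its speech-bubble lines until dialogue ends.
; Tick feeds player position into a material parameter collection for masking, and BeginPlay attaches the audio listener to the sprite.
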(event `self.ReceivePossessed`
  (params (NewController :type "Controller Object Reference"))
  (bind _asplayer_controller (cast `PlayerController` (`self.GetController`) :!label _label))
  (`EnhancedInputSubsystemInterface.AddMappingContext` (pcsubsystem `EnhancedInputLocalPlayerSubsystem` _asplayer_controller) "/Game/Input/IMC_RPG.IMC_RPG" 0 (struct)))

(event `self.ReceiveBeginPlay`
  ;[1 1 1] Initialize input system
  (`parent.ReceiveBeginPlay`)
  (`|ExecutionSequence`
    (:`then_0`
      (goto _label))
    (:`then_1`
      (`PlayerController.SetAudioListenerOverride` (`GameplayStatics.GetPlayerController` 0) (`self.Sprite`) (0.0 0.0 0.0) (struct :`Yaw` 270.0)))))

(event `self.ReceiveTick`
  (params (DeltaSeconds :type "Float (single-precision)"))
  (`parent.ReceiveTick` DeltaSeconds)
  (`KismetMaterialLibrary.SetVectorParameterValue` "/Game/Materials/MPC_Masking.MPC_Masking" "PlayerPosition" (`KismetMathLibrary.Conv_VectorToLinearColor` (`self.K2_GetActorLocation`))))

(event `EnhancedInput|/Game/Input/Actions/IA_Move`
  (params (ActionValue :type "Vector2D Structure") (ElapsedSeconds :type "Float (double-precision)") (TriggeredSeconds :type "Float (double-precision)") (InputAction :type "InputAction Object Reference" :default "/Game/Input/Actions/IA_Move.IA_Move"))
  (bind (_x _y) (`KismetMathLibrary.BreakVector2D` ActionValue))
  ;[1 1 1] Movement left, right, up, down
  (:`Triggered`
    (if (not (`self.isInteractionLocked`))
      (`self.AddMovementInput` (1.0 0.0 0.0) _x)
      (`self.AddMovementInput` (0.0 1.0 0.0) _y))))

(event `EnhancedInput|/Game/Input/Actions/IA_Interact`
  (params (ActionValue :type Boolean) (ElapsedSeconds :type "Float (double-precision)") (TriggeredSeconds :type "Float (double-precision)") (InputAction :type "InputAction Object Reference" :default "/Game/Input/Actions/IA_Interact.IA_Interact"))
  (:`Started`
    (if (`self.isInteractionLocked`)
      (if (`/Game/Widgets/WBP_SpeechBubble.FinishedRevealing` (`/Game/Widgets/WBP_HUD.WBP_SpeechBubble` (`/Game/Blueprints/GM_RPG.HUDWidget` (`self.GameMode`))))
        (bind _lastinteracted (`self.LastInteracted`)
          (:`then`
            (bind _hasnextline (message `/Game/Blueprints/Interfaces/BPI_Interaction.ShowNextLine` _lastinteracted))
            (if (not _hasnextline)
              (`self.EndInteraction`)
              (bind _lastinteracted_2 (`self.LastInteracted`)
                (:`then`
                  (message `/Game/Blueprints/Interfaces/BPI_Interaction.FinishInteraction` _lastinteracted_2)
                  (`/Game/Widgets/WBP_SpeechBubble.HideDialogue` (`/Game/Widgets/WBP_HUD.WBP_SpeechBubble` (`/Game/Blueprints/GM_RPG.HUDWidget` (`self.GameMode`)))))
                (:`else`))))
          (:`else`))
        (else
          (`/Game/Widgets/WBP_SpeechBubble.InstaReveal` (`/Game/Widgets/WBP_HUD.WBP_SpeechBubble` (`/Game/Blueprints/GM_RPG.HUDWidget` (`self.GameMode`))))))
      (else
        (for _array_element (`PrimitiveComponent.GetOverlappingActors` (`self.InteractionCheck`) null)
          (if (!= _array_element self)
            (message `/Game/Blueprints/Interfaces/BPI_Interaction.Interact` _array_element self)
            (set `self.LastInteracted` _array_element)
            (break)))))))

(fn `UserConstructionScript`
  (`parent.UserConstructionScript`))